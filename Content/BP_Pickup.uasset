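; BP_Pickup is a pickup actor that the player collects by walking into it.
; On BeginPlay it caches the third-person character and player controller, then randomly decides by weight whether it is a trigger and rolls a random health value.
; On overlap with the player, a trigger fires the character's TriggerEvent, while a normal pickup calls AddToFuse and passes itself to the controller's stat update.
; Both outcomes print a debug message and destroy the actor.
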(event EventBeginPlay
  (bind _asthird_person_character (Utilities|Casting|CastToThirdPersonCharacter (Game|Player|GetPlayerPawn 0)))
  (Variables|Default|SetTPCharacter_ref _asthird_person_character)
  (bind _asbp_player_controller (Utilities|Casting|CastToBP_PlayerController (Game|GetPlayerController 0)))
  (Variables|Default|SetBP_PlayerController_ref _asbp_player_controller)
  (Variables|Default|SetIsTrigger (Math|Random|RandomBoolwithWeight (Variables|Default|GetTriggerRatio)))
  (Variables|Default|SetHealthValue (Math|Random|RandomIntegerinRange 1 30)))

(event Collision|EventActorBeginOverlap
  (params (OtherActor :type Actor%20Object%20Reference))
  (bind _tpcharacter_ref (Variables|Default|GetTPCharacter_ref))
  (if (== OtherActor (Variables|Default|GetTPCharacter_ref))
    (if (Variables|Default|GetIsTrigger)
      (Default|TriggerEvent _tpcharacter_ref)
      (Development|PrintString "TRIGGER!" true true "(R=1.000000,G=0.000000,B=0.033410,A=1.000000)")
      (Actor|DestroyActor)
      (else
        (Default|AddtoFuse _tpcharacter_ref)
        (Default|PickUpStatUpdate (Variables|Default|GetBP_PlayerController_ref) self)
        (Development|PrintString (Utilities|String|BuildString(Integer) "" "Pickup Health Value: " (Variables|Default|GetHealthValue)))
        (Actor|DestroyActor)))))

(fn ConstructionScript)