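; Player controller that creates the HUD and manages the save slot for player health, fuse length and location.
; Game setup and respawn load the slot into controller variables, or set health and fuse defaults and write a new save if none exists.
; A sleep-save menu blocks movement and look for UI input; saving or cancelling restores game input.
; CheckHealth, CheckFuse and CheckLocation are empty stubs.
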(event Custom|StartGameSetup
  (CallFunction|SavedGameCheck))

(event Custom|Respawn
  (CallFunction|SavedGameCheck))

(event Custom|Save
  (Utilities|FlowControl|Sequence
    (:then_0
      (CallFunction|SavetheGame))
    (:then_1
      (CallFunction|ReturntoGame))))

(event Custom|SpawnSaveMenu
  (Input|SetIgnoreMoveInput true)
  (Input|SetIgnoreLookInput true)
  (Input|SetInputModeUIOnly self 0 "DoNotLock")
  (Variables|Default|SetbShowMouseCursor true)
  (Variables|Default|SetbEnableMouseOverEvents true)
  (Variables|Default|SetbEnableClickEvents true)
  (bind _returnvalue (UserInterface|CreateWidget "/Game/BP_SleepSave.BP_SleepSave_C"))
  (UserInterface|Viewport|AddtoViewport _returnvalue 0)
  (Variables|Default|SetBP_SleepSave_ref _returnvalue))

(event Custom|SaveCancelled
  (CallFunction|ReturntoGame))

(event EventBeginPlay
  (Input|SetInputModeGameOnly)
  (bind _returnvalue (UserInterface|CreateWidget "/Game/BP_HUD.BP_HUD_C"))
  (bind _output_get (Variables|Default|SetBP_HUD_ref _returnvalue))
  (UserInterface|Viewport|AddtoViewport _output_get 0)
  (bind _asthird_person_character (Utilities|Casting|CastToThirdPersonCharacter (Game|Player|GetPlayerPawn 0)))
  (Variables|Default|SetTPCharacter_ref _asthird_person_character)
  (Variables|Default|SetEnableMovement true))

(fn ConstructionScript)

(fn SavedGameCheck
  (bind _returnvalue (SaveGame|DoesSaveGameExist (Variables|Default|GetSaveSlot)))
  (if _returnvalue
    (CallFunction|LoadtheGame)
    (else
      (bind _output_get (Variables|SaveInfo|SetPlayerMaxHealth (Variables|Default|GetDefaultMaxHealth)))
      (Variables|Default|SetCurrentHealth _output_get)
      (Variables|Default|SetCurrentFuseLength (Variables|Default|GetDefaultFuseLength))
      (CallFunction|SavetheGame))))

(fn SavetheGame
  (bind _returnvalue (SaveGame|CreateSaveGameObject "/Game/BP_SaveGame.BP_SaveGame_C"))
  (bind _asbp_save_game (Utilities|Casting|CastToBP_SaveGame _returnvalue))
  (bind _output_get (Variables|Default|SetBP_SaveGame_ref _asbp_save_game))
  (Variables|/Game/BP_SaveGame.BP_SaveGame_C|SetSavedMaxHealth _output_get (Variables|SaveInfo|GetPlayerMaxHealth))
  (Variables|/Game/BP_SaveGame.BP_SaveGame_C|SetSavedCurrentHealth _output_get (Variables|SaveInfo|GetSavedPlayerHealth))
  (Variables|/Game/BP_SaveGame.BP_SaveGame_C|SetSavedFuseLength _output_get (Variables|SaveInfo|GetSavedFuseLength))
  (Variables|/Game/BP_SaveGame.BP_SaveGame_C|SetSavedLocation _output_get (Variables|SaveInfo|GetSavedLocation))
  (SaveGame|SaveGametoSlot (Variables|Default|GetBP_SaveGame_ref) (Variables|Default|GetSaveSlot)))

(fn CheckHealth)

(fn CheckFuse)

(fn CheckLocation)

(fn LoadtheGame
  (bind _returnvalue (SaveGame|LoadGamefromSlot (Variables|Default|GetSaveSlot)))
  (bind _asbp_save_game (Utilities|Casting|CastToBP_SaveGame _returnvalue))
  (Variables|SaveInfo|SetPlayerMaxHealth (Variables|/Game/BP_SaveGame.BP_SaveGame_C|GetSavedMaxHealth _asbp_save_game))
  (Variables|SaveInfo|SetSavedPlayerHealth (Variables|/Game/BP_SaveGame.BP_SaveGame_C|GetSavedCurrentHealth _asbp_save_game))
  (Variables|SaveInfo|SetSavedFuseLength (Variables|/Game/BP_SaveGame.BP_SaveGame_C|GetSavedFuseLength _asbp_save_game))
  (Variables|SaveInfo|SetSavedLocation (Variables|/Game/BP_SaveGame.BP_SaveGame_C|GetSavedLocation _asbp_save_game)))

(fn ReturntoGame
  (Input|SetInputModeGameOnly self)
  (Variables|Default|SetbShowMouseCursor false)
  (Variables|Default|SetbEnableMouseOverEvents false)
  (Variables|Default|SetbEnableClickEvents false)
  (Input|ResetIgnoreMoveInput)
  (Input|ResetIgnoreLookInput)
  (Class|Controller|ResetIgnoreInputFlags)
  (Widget|RemovefromParent (Variables|Default|GetBP_SleepSave_ref)))