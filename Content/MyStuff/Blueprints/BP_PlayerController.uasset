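; Player controller that owns the HUD, player health, sleep-save menu and respawning.
; A looping one-second timer drains health, pickups restore it up to max, and flashbacks pause the drain.
; Saves store location plus health and fuse values, kept in variables separate from the live health, and the slot is deleted on EndPlay.
; Respawn reloads the save, teleports the character above the saved location, restarts the drain and flags bed overlap.
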(event Custom|StartGameSetup
  (CallFunction|SavedGameCheck))

(event Custom|Respawn
  (bind _savedlocation (Variables|SaveInfo|GetSavedLocation))
  (bind _tpcharacter_ref (Variables|Default|GetTPCharacter_ref))
  (Utilities|FlowControl|Sequence
    (:then_0
      (CallFunction|SavedGameCheck))
    (:then_1
      (Default|Respawn (Variables|Default|GetTPCharacter_ref)))
    (:then_2
      (Transformation|AttachComponentToComponent (Variables|/Script/Engine.Character|GetMesh _tpcharacter_ref) (Variables|/Script/Engine.Character|GetCapsuleComponent _tpcharacter_ref) "None" "KeepWorld" "KeepWorld" "SnapToTarget" true)
      (Transformation|SetActorTransform (Variables|Default|GetTPCharacter_ref) (Math|Transform|MakeTransform (Math|Vector|MakeVector (.x _savedlocation) (.y _savedlocation) (+ (.z _savedlocation) 2e+02)) "0, 0, 0" "1,1,1") false true)
      (Input|SetIgnoreMoveInput false)
      (Utilities|Time|SetTimerbyFunctionName self "TickDecreaseHealth" 1.0 true)
      (Default|Respawn (Variables|Default|GetBP_HUD_ref)))
    (:then_3
      (if (== (Utilities|Array|Get(acopy) (Collision|GetOverlappingActors (Variables|/Script/Engine.Character|GetCapsuleComponent (Variables|Default|GetTPCharacter_ref)) "/Game/MyStuff/Blueprints/BP_Bed.BP_Bed_C" :!class /Script/Engine.PrimitiveComponent)) "/Game/MyStuff/Blueprints/BP_Bed.BP_Bed")
        (Variables|Default|SetbRespawnedAtSavePoint true)
        (else
          (Variables|Default|SetbRespawnedAtSavePoint false))))))

(event Custom|Save
  (Variables|SaveInfo|SetSavedLocation (Variables|Default|GetCurrentLocation))
  (Utilities|FlowControl|Sequence
    (:then_0
      (CallFunction|SavetheGame))
    (:then_1
      (CallFunction|ReturntoGame))))

(event Custom|SpawnSaveMenu
  (Input|SetIgnoreMoveInput true)
  (Input|SetIgnoreLookInput true)
  (Input|SetInputModeUIOnly self 0 "DoNotLock")
  (Variables|Default|SetbShowMouseCursor true)
  (Variables|Default|SetbEnableMouseOverEvents true)
  (Variables|Default|SetbEnableClickEvents true)
  (bind _returnvalue (UserInterface|CreateWidget "/Game/MyStuff/Blueprints/BP_SleepSave.BP_SleepSave_C"))
  (UserInterface|Viewport|AddtoViewport _returnvalue 0)
  (Variables|Default|SetBP_SleepSave_ref _returnvalue))

(event Custom|SaveCancelled
  (CallFunction|ReturntoGame))

(event Custom|PlayerController_Flashback
  (Class|KismetSystemLibrary|PauseTimer 0 "TickDecreaseHealth"))

(event Custom|PickUpStatUpdate
  (params (BP_PickUp_ref :type BP%20Pickup%20Object%20Reference))
  (bind _healthvalue (Variables|/Game/MyStuff/Blueprints/BP_Pickup.BP_Pickup_C|GetHealthValue BP_PickUp_ref))
  (bind _returnvalue (Math|Conversions|ToFloat(Integer) _healthvalue))
  (Class|KismetSystemLibrary|PauseTimer self "TickDecreaseHealth")
  (if (< (- (Variables|Default|GetCurrentMaxHealth) (Variables|Default|GetCurrentHealth)) _returnvalue)
    (Variables|Default|SetCurrentHealth (Variables|Default|GetCurrentMaxHealth))
    (else
      (Variables|Default|SetCurrentHealth (+ (Variables|Default|GetCurrentHealth) _returnvalue))))
  (Class|KismetSystemLibrary|UnPauseTimer self "TickDecreaseHealth"))

(event EventBeginPlay
  (bind _self self)
  (Input|SetInputModeGameOnly _self)
  (bind _returnvalue (UserInterface|CreateWidget "/Game/MyStuff/Blueprints/BP_HUD.BP_HUD_C" _self))
  (bind _output_get (Variables|Default|SetBP_HUD_ref _returnvalue))
  (UserInterface|Viewport|AddtoViewport _output_get 0)
  (bind _asthird_person_character (Utilities|Casting|CastToThirdPersonCharacter (Game|Player|GetPlayerPawn 0)))
  (Variables|Default|SetTPCharacter_ref _asthird_person_character)
  (Variables|Default|SetEnableMovement true)
  (Variables|Default|SetbRespawnedAtSavePoint false)
  (Utilities|Time|SetTimerbyFunctionName self "TickDecreaseHealth" 1.0 true)
  (CallFunction|SavedGameCheck))

(event EventTick
  (params (DeltaSeconds :type Float%20%28single-precision%29))
  (Variables|Default|SetCurrentLocation (Transformation|GetActorLocation (Variables|Default|GetTPCharacter_ref))))

(event EventEndPlay
  (params (EndPlayReason :type EEndPlayReason%20Enum :default "Destroyed"))
  (SaveGame|DeleteGameinSlot (Variables|Default|GetSaveSlot)))

(fn ConstructionScript)

(fn SavedGameCheck
  (bind _returnvalue (SaveGame|DoesSaveGameExist (Variables|Default|GetSaveSlot)))
  (if _returnvalue
    (CallFunction|LoadtheGame)
    (else
      (bind _output_get (Variables|Default|SetCurrentMaxHealth (Variables|Default|GetDefaultMaxHealth)))
      (Variables|Default|SetCurrentHealth _output_get)
      (Variables|Default|SetCurrentFuseLength (Variables|Default|GetDefaultFuseLength))
      (Variables|SaveInfo|SetSavedLocation (Transformation|GetActorLocation (Class|GameModeBase|FindPlayerStart (Game|GetGameMode))))
      (bind _returnvalue_2 (SaveGame|CreateSaveGameObject "/Game/MyStuff/Blueprints/BP_SaveGame.BP_SaveGame_C"))
      (bind _asbp_save_game (Utilities|Casting|CastToBP_SaveGame _returnvalue_2))
      (Variables|Default|SetBP_SaveGame_ref _asbp_save_game)
      (CallFunction|SavetheGame))))

(fn SavetheGame
  (bind _bp_savegame_ref (Variables|Default|GetBP_SaveGame_ref))
  (Variables|/Game/MyStuff/Blueprints/BP_SaveGame.BP_SaveGame_C|SetSavedMaxHealth _bp_savegame_ref (Variables|SaveInfo|GetPlayerMaxHealth))
  (Variables|/Game/MyStuff/Blueprints/BP_SaveGame.BP_SaveGame_C|SetSavedCurrentHealth _bp_savegame_ref (Variables|SaveInfo|GetSavedPlayerHealth))
  (Variables|/Game/MyStuff/Blueprints/BP_SaveGame.BP_SaveGame_C|SetSavedFuseLength _bp_savegame_ref (Variables|SaveInfo|GetSavedFuseLength))
  (bind _output_get (Variables|/Game/MyStuff/Blueprints/BP_SaveGame.BP_SaveGame_C|SetSavedLocation _bp_savegame_ref (Variables|SaveInfo|GetSavedLocation)))
  (SaveGame|SaveGametoSlot (Variables|Default|GetBP_SaveGame_ref) (Variables|Default|GetSaveSlot)))

(fn CheckHealth)

(fn CheckFuse)

(fn CheckLocation)

(fn LoadtheGame
  (bind _returnvalue (SaveGame|LoadGamefromSlot (Variables|Default|GetSaveSlot)))
  (bind _asbp_save_game (Utilities|Casting|CastToBP_SaveGame _returnvalue))
  (Variables|SaveInfo|SetPlayerMaxHealth (Variables|/Game/MyStuff/Blueprints/BP_SaveGame.BP_SaveGame_C|GetSavedMaxHealth _asbp_save_game))
  (Variables|SaveInfo|SetSavedPlayerHealth (Variables|/Game/MyStuff/Blueprints/BP_SaveGame.BP_SaveGame_C|GetSavedCurrentHealth _asbp_save_game))
  (Variables|SaveInfo|SetSavedFuseLength (Variables|/Game/MyStuff/Blueprints/BP_SaveGame.BP_SaveGame_C|GetSavedFuseLength _asbp_save_game))
  (Variables|SaveInfo|SetSavedLocation (Variables|/Game/MyStuff/Blueprints/BP_SaveGame.BP_SaveGame_C|GetSavedLocation _asbp_save_game)))

(fn ReturntoGame
  (Input|SetInputModeGameOnly self)
  (Variables|Default|SetbShowMouseCursor false)
  (Variables|Default|SetbEnableMouseOverEvents false)
  (Variables|Default|SetbEnableClickEvents false)
  (Input|ResetIgnoreMoveInput)
  (Input|ResetIgnoreLookInput)
  (Class|Controller|ResetIgnoreInputFlags)
  (Widget|RemovefromParent (Variables|Default|GetBP_SleepSave_ref)))

(fn TickDecreaseHealth
  (bind _result (Math|Float|DecrementFloat (Variables|Default|GetCurrentHealth))
    (:%20%20
      (bind _output_get (Variables|Default|SetCurrentHealth _result))
      (Development|PrintString (Utilities|String|BuildString(Float) "" "Current Health: " _output_get)))))