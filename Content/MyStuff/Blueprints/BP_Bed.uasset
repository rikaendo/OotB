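; BP_Bed is a save-point bed that opens the save menu when the player character overlaps its collision box.
; It caches the character and BP_PlayerController on BeginPlay and mirrors the controller's RespawnedAtSavePoint flag every Tick.
; With an existing save, that flag suppresses the menu after respawning at a save point.
; Any end overlap on the box clears the controller's flag, without checking which actor left.
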(event OnComponentBeginOverlap(collision_Box)
  (params (OverlappedComponent :type Primitive%20Component%20Object%20Reference) (OtherActor :type Actor%20Object%20Reference) (OtherComp :type Primitive%20Component%20Object%20Reference) (OtherBodyIndex :type Integer) (bFromSweep :type Boolean) (SweepResult :type Hit%20Result%20Structure%20%28by%20ref%29))
  (bind _bp_playercontroller_ref (Variables|Default|GetBP_PlayerController_ref))
  (if (== OtherActor (Variables|Default|GetTPCharacter_ref))
    (bind _returnvalue (SaveGame|DoesSaveGameExist (Variables|/Game/MyStuff/Blueprints/BP_PlayerController.BP_PlayerController_C|GetSaveSlot (Variables|Default|GetBP_PlayerController_ref))))
    (if _returnvalue
      (if (not (Variables|Default|GetbRespawnedAtSavePoint))
        (Default|SpawnSaveMenu _bp_playercontroller_ref))
      (else
        (Default|SpawnSaveMenu _bp_playercontroller_ref)))))

(event OnComponentEndOverlap(collision_Box)
  (params (OverlappedComponent :type Primitive%20Component%20Object%20Reference) (OtherActor :type Actor%20Object%20Reference) (OtherComp :type Primitive%20Component%20Object%20Reference) (OtherBodyIndex :type Integer))
  (Variables|/Game/MyStuff/Blueprints/BP_PlayerController.BP_PlayerController_C|SetbRespawnedAtSavePoint (Variables|Default|GetBP_PlayerController_ref) false))

(event EventBeginPlay
  (bind _asthird_person_character (Utilities|Casting|CastToThirdPersonCharacter (Game|Player|GetPlayerPawn 0)))
  (Variables|Default|SetTPCharacter_ref _asthird_person_character)
  (bind _asbp_player_controller (Utilities|Casting|CastToBP_PlayerController (Game|GetPlayerController 0)))
  (Variables|Default|SetBP_PlayerController_ref _asbp_player_controller))

(event EventTick
  (params (DeltaSeconds :type Float%20%28single-precision%29))
  (Variables|Default|SetbRespawnedAtSavePoint (Variables|/Game/MyStuff/Blueprints/BP_PlayerController.BP_PlayerController_C|GetbRespawnedAtSavePoint (Variables|Default|GetBP_PlayerController_ref))))

(fn ConstructionScript)